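; Game mode that runs endless numbered waves of spider enemies, starting shortly after play begins.
; Each wave resets a fixed spawn count and sets a non-looping timer for SpawnSpider, which tracks results in SpiderArray.
; RegisterSpiderDeath removes spiders and starts the next wave after a delay once none remain alive or pending.
; EnemySpawn only gathers TargetPoints; its random-point spawn and return, plus difficulty scaling, are unwired.
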(event `self.ReceiveBeginPlay`
  (`KismetSystemLibrary.Delay` 2.0)
  (`self.StartNewWave`))

(event `SpawnSpider`
  (bind _returnvalue (`self.Enemy Spawn`))
  (`KismetArrayLibrary.Array_Add` (`self.SpiderArray`) _returnvalue)
  (bind _result (`/Engine/EditorBlueprintResources/StandardMacros.DecrementInt` (`self.SpiderRemaningToSpawn`))
    (:`  `
      (bind _output_get (set `self.SpiderRemaningToSpawn` _result))
      (if (== _output_get 0)
        (`KismetSystemLibrary.K2_ClearTimer` null "SpawnSpider")))))

(event `End Wave`
  (`KismetSystemLibrary.Delay` 2.0)
  (`self.StartNewWave`))

(fn `Enemy Spawn`
  (returns (ReturnValue :type "/Game/Blueprints/BP_Spider_01 Object Reference"))
  (bind _outactors (`GameplayStatics.GetAllActorsOfClass` "/Script/Engine.TargetPoint")))

(fn `Register Spider Death`
  (params (Item :type "/Game/Blueprints/BP_Spider_01 Object Reference (by ref)"))
  (bind _spiderarray (`self.SpiderArray`))
  (`KismetArrayLibrary.Array_RemoveItem` _spiderarray Item)
  (if (and (== (`KismetArrayLibrary.Array_Length` _spiderarray) 0) (== (`self.SpiderRemaningToSpawn`) 0))
    (`self.End Wave`)))

(fn `StartNewWave`
  (`/Engine/EditorBlueprintResources/StandardMacros.IncrementInt` (`self.WaveNumber`)
    (:`  `
      (set `self.SpiderRemaningToSpawn` 2)
      (`KismetSystemLibrary.K2_SetTimer` null "SpawnSpider" 2.0))))

(fn `UserConstructionScript`)