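; Playable soldier for what appears to be a twin-stick style shooter, creating its HUD on BeginPlay and tracking health until death.
; Movement follows world axes, while control rotation eases toward the mouse's motion direction once its velocity exceeds a dead zone.
; Left mouse toggles muzzle effect and sound, with immediate and timer-driven debug-drawn line traces from the muzzle socket applying damage.
; Death blocks movement, turning and new shots.
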(event `self.ReceiveBeginPlay`
  ;[0.1783 0.626 0.2204] UI
  (bind _returnvalue (`|CreateWidget` "/Game/UI/W_PlayerHUD.W_PlayerHUD_C" null self))
  (`UserWidget.AddToViewport` _returnvalue 0))

(event `self.ReceiveTick`
  (params (DeltaSeconds :type "Float (single-precision)"))
  ;[0.1475 0.8701 1] Player Rotation
  (if (not (`self.Dead`))
    (`self.UpdatePlayerRotation`)))

(event `self.ReceiveAnyDamage`
  (params (Damage :type "Float (single-precision)") (DamageType :type "DamageType Object Reference") (InstigatedBy :type "Controller Object Reference") (DamageCauser :type "Actor Object Reference"))
  ;[0.2594 0.02567 0.02567] Damage System
  (`self.ApplyDamageToPlayer` Damage))

(event `InputAxis|MoveBack`
  (params (AxisValue :type "Float (single-precision)"))
  ;[0.09894 0.2439 1] Marine movements
  (if (not (`self.Dead`))
    (`self.AddMovementInput` (`KismetMathLibrary.MakeVector` AxisValue))))

(event `InputAxis|MoveLeftRight`
  (params (AxisValue :type "Float (single-precision)"))
  ;[0.09894 0.2439 1] Marine movements
  (if (not (`self.Dead`))
    (`self.AddMovementInput` (`KismetMathLibrary.MakeVector` 0.0 AxisValue))))

(event `Key|LeftMouseButton`
  (params (Key :type "Key Structure"))
  ;[1 0.1469 0.05326] Weapon Effect Fire
  (:`Pressed`
    (if (not (`self.Dead`))
      (`self.ClickedToFire`)
      (`self.GenerateLineTrance`)
      (`KismetSystemLibrary.K2_SetTimer` null "GenerateLineTrance" 0.08)))
  (:`Released`
    (`self.StopFire`)
    (`KismetSystemLibrary.K2_ClearTimer` null "GenerateLineTrance")))

(fn `ApplyDamageToPlayer`
  (params (Damage :type "Float (double-precision)"))
  (returns (IsPlayerDead :type Boolean))
  (bind _output_get (set `self.Health` (- (`self.Health`) Damage)))
  (if (== (`KismetMathLibrary.FClamp` _output_get 0.0 100.0) 0.0)
    (bind _output_get_2 (set `self.Dead` true))
    (return _output_get_2)))

(fn `ClickedToFire`
  (`ActorComponent.Activate` (`self.P_AssaultRifle_MF`) false)
  (bind _returnvalue (`GameplayStatics.SpawnSound2D` "/Game/Sounds/Weapon_AssaultRifle/Stereo/AssaultRifle_LoopShoot_Cue.AssaultRifle_LoopShoot_Cue" 1.0 1.0 0.0 null))
  (set `self.WeaponFireSound` _returnvalue))

(fn `EndLocationLineTrace`
  (returns (ReturnValue :type "Vector Structure"))
  (return (+ (* (`KismetMathLibrary.GetForwardVector` (`SceneComponent.GetSocketRotation` (`self.P_AssaultRifle_MF`) "MuzzleFlashSocket")) 2000.0) (`self.StartLocationLineTrace`))))

(fn `GenerateLineTrance`
  (bind _outhit (`KismetSystemLibrary.LineTraceSingle` :`Start` (`self.StartLocationLineTrace`) :`End` (`self.EndLocationLineTrace`) :`TraceChannel` "TraceTypeQuery1" :`DrawDebugType` "ForDuration"))
  (bind (_bblockinghit _binitialoverlap _time _distance _location _impactpoint _normal _impactnormal _physmat _hitactor) (`GameplayStatics.BreakHitResult` _outhit))
  (if _bblockinghit
    (`GameplayStatics.ApplyDamage` _hitactor (`self.Base Damage`))))

(fn `GetMouseVelocity`
  (returns (ReturnValue :type "Vector2D Structure"))
  (bind (_deltax _deltay) (`PlayerController.GetInputMouseDelta` (`GameplayStatics.GetPlayerController` 0)))
  (return (/ (`KismetMathLibrary.MakeVector2D` _deltax _deltay) (`GameplayStatics.GetWorldDeltaSeconds`))))

(fn `IsMouseDeadZone`
  (returns (ReturnValue :type Boolean))
  (return (> (`KismetMathLibrary.VSize2D` (`self.GetMouseVelocity`)) (`self.MouseDeadZone`))))

(fn `StartLocationLineTrace`
  (returns (ReturnValue :type "Vector Structure"))
  (return (`SceneComponent.GetSocketLocation` (`self.P_AssaultRifle_MF`) "MuzzleFlashSocket")))

(fn `StopFire`
  (`ActorComponent.Deactivate` (`self.P_AssaultRifle_MF`))
  (if (not (`self.Dead`))
    (`AudioComponent.StopDelayed` (`self.WeaponFireSound`) 0.0)
    (`/Engine/EditorBlueprintResources/StandardMacros.IsValid` "/Game/Sounds/Weapon_AssaultRifle/Stereo/AssaultRifle_EndShoot_Cue.AssaultRifle_EndShoot_Cue"
      (:`Is Valid`
        (`GameplayStatics.SpawnSound2D` "/Game/Sounds/Weapon_AssaultRifle/Stereo/AssaultRifle_EndShoot_Cue.AssaultRifle_EndShoot_Cue" 1.0 1.0 0.0 null)))))

(fn `UpdatePlayerRotation`
  (locals (NewLocalVar_0 :type "Vector2D Structure"))
  (bind (_returnvalue_x _returnvalue_y) (`KismetMathLibrary.BreakVector2D` (`self.GetMouseVelocity`)))
  (bind _returnvalue (`GameplayStatics.GetPlayerController` 0))
  (if (`self.IsMouseDeadZone`)
    (`Controller.SetControlRotation` _returnvalue (`KismetMathLibrary.RInterpTo` (`Controller.GetControlRotation` _returnvalue) (`KismetMathLibrary.MakeRotator` 0.0 0.0 (`KismetMathLibrary.DegAtan2` _returnvalue_x _returnvalue_y)) (`GameplayStatics.GetWorldDeltaSeconds`) 7.0))))

(fn `UserConstructionScript`)