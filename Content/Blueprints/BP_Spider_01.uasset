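; BP_Spider_01 is a spider enemy that chases the player and plays a melee attack montage up close.
; From BeginPlay an AI MoveTo toward the player character loops, reissuing shortly after each success or failure.
; Each Tick, if the soldier player is in close range and no attack is playing, it deactivates CharacterMovement and plays the attack, reactivating movement when the montage completes.
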(event `self.ReceiveBeginPlay`
  ;[1 0.6703 0.1612] Spider Movement
  (`|AIMoveTo` self (0.0 0.0 0.0) (`GameplayStatics.GetPlayerCharacter` 0) :!label _label
    (:`OnSuccess`
      _)
    (:`OnFail`
      _))
  (`KismetSystemLibrary.Delay` 0.2)
  (goto _label))

(event `self.ReceiveTick`
  (params (DeltaSeconds :type "Float (single-precision)"))
  ;[1 0.1401 0.1899] Spider Attack
  (if (and (`self.IsAttackRange`) (not (`self.IsAttacking`)))
    (`self.SpiderMovementDeactivate`)
    (`|PlayMontage` (`self.Mesh`) "/Game/Characters/Enemy_Great_Spider/Animations/AM_Spider_Attack.AM_Spider_Attack" 1.5
      (:`OnCompleted`
        (`self.SpiderMovementActive`)))))

(fn `IsAttacking`
  (returns (ReturnValue :type Boolean))
  (return (`AnimInstance.Montage_IsPlaying` (`SkeletalMeshComponent.GetAnimInstance` (`self.Mesh`)) "/Game/Characters/Enemy_Great_Spider/Animations/AM_Spider_Attack.AM_Spider_Attack")))

(fn `IsAttackRange`
  (returns (ReturnValue :type Boolean))
  (bind _asbp_soldier_01 (cast `/Game/Blueprints/BP_Soldier_01` (`GameplayStatics.GetPlayerPawn` 0)))
  (return (< (`self.GetDistanceTo` _asbp_soldier_01) 100.0)))

(fn `SpiderMovementActive`
  (`ActorComponent.Activate` (`self.CharacterMovement`) false))

(fn `SpiderMovementDeactivate`
  (`ActorComponent.Deactivate` (`self.CharacterMovement`)))

(fn `UserConstructionScript`)